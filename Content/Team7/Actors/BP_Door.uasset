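; Two-part sliding door actor that opens, closes or toggles through custom events gated by CanOpenDoor.
; BeginPlay derives each part's open position by offsetting its pivot along local X by the mesh's bounds width, and snaps there if IsDoorOpen is set.
; Separate open and close timelines lerp both pivots and update IsDoorOpen, with play rates scaled by DoorsOpeningDuration.
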(event Custom|CE_CloseDoor
  ;[0.15 0.15 0.15 0.5] Event that close doors with the help of a timeline
  (if (Variables|Default|GetCanOpenDoor)
    (bind _alpha (Timeline|CloseDoors Play)
      (:Update
        ;[0.15 0.15 0.15 0.5] The vectors are used to update the position of the 2 parts
        (Transformation|SetRelativeLocation (Variables|Default|GetLeftPartPivot) (Math|Vector|Lerp(Vector) (Variables|Default|GetLeftEnd) (Variables|Default|GetLeftStart) _alpha) false false)
        (Transformation|SetRelativeLocation (Variables|Default|GetRightPartPivot) (Math|Vector|Lerp(Vector) (Variables|Default|GetRightEnd) (Variables|Default|GetRightStart) _alpha) false false)
        (Variables|Default|SetIsDoorOpen false)))))

(event Custom|CE_OpenDoors
  ;[0.15 0.15 0.15 0.5] Event that open doors with the help of a timeline
  (if (Variables|Default|GetCanOpenDoor)
    (bind _alpha (Timeline|OpenDoors Play)
      (:Update
        ;[0.15 0.15 0.15 0.5] The vectors are used to update the position of the 2 parts
        (Transformation|SetRelativeLocation (Variables|Default|GetLeftPartPivot) (Math|Vector|Lerp(Vector) (Variables|Default|GetLeftStart) (Variables|Default|GetLeftEnd) _alpha) false false)
        (Transformation|SetRelativeLocation (Variables|Default|GetRightPartPivot) (Math|Vector|Lerp(Vector) (Variables|Default|GetRightStart) (Variables|Default|GetRightEnd) _alpha) false false)
        (Variables|Default|SetIsDoorOpen true)))))

(event Custom|CE_ActionDoors
  ;[0.15 0.15 0.15 0.5] Event that close or open doors depending on the current state
  (if (Variables|Default|GetCanOpenDoor)
    (if (Variables|Default|GetIsDoorOpen)
      (CallFunction|CECloseDoor)
      (else
        (CallFunction|CEOpenDoors)))))

(event EventBeginPlay
  (bind _rightpart (Variables|Default|GetRightPart))
  (bind _leftpartpivot (Variables|Default|GetLeftPartPivot))
  (bind _rightpartpivot (Variables|Default|GetRightPartPivot))
  (bind _leftpart (Variables|Default|GetLeftPart))
  (bind (_min _max) (Components|StaticMesh|GetLocalBounds _rightpart))
  (bind (_min_2 _max_2) (Components|StaticMesh|GetLocalBounds _leftpart))
  (bind _relativelocation (Variables|/Script/Engine.SceneComponent|GetRelativeLocation _leftpartpivot))
  (bind _relativelocation_2 (Variables|/Script/Engine.SceneComponent|GetRelativeLocation _rightpartpivot))
  ;[0.15 0.15 0.15 0.5] Left part : save Originx and OffsetX
  (Variables|Default|SetCanOpenDoor true)
  (Variables|Default|SetLeftStart (Variables|/Script/Engine.SceneComponent|GetRelativeLocation _leftpartpivot))
  (Variables|Default|SetLeftEnd (Math|Vector|MakeVector (- (.x _relativelocation) (.x (- _max_2 _min_2))) (.y _relativelocation) (.z _relativelocation)))
  ;[0.15 0.15 0.15 0.5] Right Part : save OriginX and OffsetX
  (Variables|Default|SetRightStart (Variables|/Script/Engine.SceneComponent|GetRelativeLocation _rightpartpivot))
  (Variables|Default|SetRightEnd (Math|Vector|MakeVector (+ (.x _relativelocation_2) (.x (- _max _min))) (.y _relativelocation_2) (.z _relativelocation_2)))
  ;[0.15 0.15 0.15 0.5] Set the time that the door will take to open/close
  (Components|Timeline|SetPlayRate (Variables|Default|GetOpenDoors) (/ 1.0 (Variables|Default|GetDoorsOpeningDuration)))
  (Components|Timeline|SetPlayRate (Variables|Default|GetCloseDoors) (/ 1.0 (Variables|Default|GetDoorsOpeningDuration)))
  ;[0.15 0.15 0.15 0.5] If the door is initially open : reposition the parts
  (if (Variables|Default|GetIsDoorOpen)
    (Transformation|SetRelativeLocation (Variables|Default|GetLeftPartPivot) (Variables|Default|GetLeftEnd) false false)
    (Transformation|SetRelativeLocation (Variables|Default|GetRightPartPivot) (Variables|Default|GetRightEnd) false false)))

(fn ConstructionScript)