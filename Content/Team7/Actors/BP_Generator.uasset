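; BP_Generator is an interactable generator actor that, when switched off, removes a linked water death zone.
; It plays a generator-on sound at its audio origin on BeginPlay.
; While active it supplies a deactivation prompt to the interaction UI, and interacting destroys the linked WaterDeathZone and sets IsDesactivated, which blanks the prompt.
; Without a linked zone the interaction changes nothing, and deactivation leaves the sound untouched.
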(event EventBeginPlay
  (Audio|PlaySoundatLocation "/Game/FirstPerson/SoundDesign/MetaSounds/Loop/MS_LP_GeneratorON.MS_LP_GeneratorON" (Transformation|GetWorldLocation (Variables|Default|GetAudioOrigin)) "0, 0, 0" 1.0 1.0 0.0 0 0 0 0))

(event EventShowInteraction
  (params (InteractUI :type WBP%20Interaction%20Object%20Reference))
  ;[0.15 0.15 0.15 0.5] Show intercation message when still activated
  (if (Variables|Default|GetIsDesactivated)
    (Default|SetInteractMessage InteractUI)
    (else
      (Default|SetInteractMessage InteractUI "Press [E] to desactivate generator"))))

(event EventInteract
  ;[0.15 0.15 0.15 0.5] If the corresponding Deathzone is linked, destroy the Deathzone
  (if (not (Variables|Default|GetIsDesactivated))
    (if (!= (Variables|Default|GetWaterDeathZone) 0)
      (Actor|DestroyActor (Variables|Default|GetWaterDeathZone))
      (Variables|Default|SetIsDesactivated true))))

(fn ConstructionScript)