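; BP_Lever is an interactable lever actor that takes part in what appears to be an ordered activation puzzle.
; It shows its configured message on the interaction UI, and on interaction marks itself active and fires the ActivateTimer dispatcher with its index and itself.
; A custom deactivate event resets it, with a debug message indicating it was pulled out of order.
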(event Custom|CE_Desactivate
  (Variables|Default|SetActivate false)
  (Development|PrintString "Désactivé pas dans l'ordre"))

(event EventBeginPlay)

(event Collision|EventActorBeginOverlap
  (params (OtherActor :type Actor%20Object%20Reference)))

(event EventTick
  (params (DeltaSeconds :type Float%20%28single-precision%29)))

(event EventShowInteraction
  (params (InteractUI :type WBP%20Interaction%20Object%20Reference))
  (Default|SetInteractMessage InteractUI (Variables|Default|GetSet%20Message%20to%20Show)))

(event EventInteract
  (Variables|Default|SetActivate true)
  (Default|CallActivateTimer (Variables|Default|GetIndexNumber) self)
  (Development|PrintString "Activé"))

(fn ConstructionScript)