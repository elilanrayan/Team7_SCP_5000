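; BP_Password is an interactable password terminal that opens its linked door once the correct password is entered.
; Interacting creates a WBP_Password widget through the HUD held by the GI_SCP game instance, passing it the expected password and binding its close and validate events.
; Validation, if the door can open, triggers the door, plays a success sound and closes the widget.
; The terminal then stops showing its prompt and ignores further interaction.
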(event Custom|CE_ValidateWidget
  ;[0.15 0.15 0.15 0.5] Validate Widget : Open the corresponding door then close widget
  (if (!= (Variables|Default|GetDoor) 0)
    (if (Variables|/Game/Team7/Actors/BP_Door.BP_Door_C|GetCanOpenDoor (Variables|Default|GetDoor))
      (Variables|Default|SetIsValidated true)
      (Default|CEActionDoors (Variables|Default|GetDoor))
      (Audio|PlaySoundatLocation "/Game/FirstPerson/SoundDesign/MetaSounds/OneShot/MS_OS_GoodPassword.MS_OS_GoodPassword" (Transformation|GetWorldLocation (Variables|Default|GetAudioOrigin)) "0, 0, 0" 1.0 1.0 0.0 0 0 0 0)
      (CallFunction|CECloseWidget))))

(event Custom|CE_CloseWidget
  ;[0.15 0.15 0.15 0.5] Close Password Widegt
  (Variables|Default|SetIsOpened (not (Variables|Default|GetIsOpened)))
  (if (Variables|Default|GetGI%20IsValid)
    (Default|CEReturntoGame (Variables|/Game/Team7/Game/GI_SCP.GI_SCP_C|GetHUD (Variables|Default|GetAs%20GI%20SCP)) (Variables|Default|GetPasswordUI))))

(event EventBeginPlay
  ;[0.15 0.15 0.15 0.5] BeginPlay
  (bind _asgi_scp (Utilities|Casting|CastToGI_SCP (Game|GetGameInstance)))
  (bind _output_get (Variables|Default|SetAs%20GI%20SCP _asgi_scp))
  (if (!= _output_get 0)
    (Variables|Default|SetGI%20IsValid true)
    (else
      (Variables|Default|SetGI%20IsValid false))))

(event EventShowInteraction
  (params (InteractUI :type WBP%20Interaction%20Object%20Reference))
  ;[0.15 0.15 0.15 0.5] Show interaction message depending if the Password Widget is open
  (if (or (Variables|Default|GetIsOpened) (Variables|Default|GetIsValidated))
    (Default|SetInteractMessage InteractUI)
    (else
      (Default|SetInteractMessage InteractUI "Press [E] to enter password"))))

(event EventInteract
  (bind _as_gi_scp (Variables|Default|GetAs%20GI%20SCP))
  (bind _hud (Variables|/Game/Team7/Game/GI_SCP.GI_SCP_C|GetHUD _as_gi_scp))
  ;[0.15 0.15 0.15 0.5] Creating, setting up and opening Password Widget
  (if (not (Variables|Default|GetIsValidated))
    (Variables|Default|SetIsOpened (not (Variables|Default|GetIsOpened)))
    (if (Variables|Default|GetGI%20IsValid)
      (Default|CEInteractableUI _hud)
      (bind _wbpcreate (Default|FCreateWBP _hud "/Game/Team7/UI/WBP_Password.WBP_Password_C"))
      (bind _aswbp_password (Utilities|Casting|CastToWBP_Password _wbpcreate))
      (Variables|Default|SetPasswordUI _aswbp_password)
      (EventDispatchers|BindEventtoCloseWidget (Variables|Default|GetPasswordUI) (EventDispatchers|CreateEvent :!event Custom|CE_CloseWidget))
      (EventDispatchers|BindEventtoValidateWidget (Variables|Default|GetPasswordUI) (EventDispatchers|CreateEvent :!event Custom|CE_ValidateWidget))
      (Variables|/Game/Team7/UI/WBP_Password.WBP_Password_C|SetExcpectedPassword (Variables|Default|GetPasswordUI) (Variables|Default|GetExcpectedPassword)))))

(fn ConstructionScript)