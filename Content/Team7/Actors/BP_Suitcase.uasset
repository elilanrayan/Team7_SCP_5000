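; BP_Suitcase is an interactable suitcase pickup that shows a press-E prompt through the interaction UI.
; On interact it has the first-person character add a mapping context, noted as carrying the Reset Run input action, then destroys itself and sets HasSuitcase on the GI_SCP game instance.
; On BeginPlay it reads that flag and destroys itself if the suitcase is already held.
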(event EventBeginPlay
  (bind _asgi_scp (Utilities|Casting|CastToGI_SCP (Game|GetGameInstance)))
  (bind _output_get (Variables|Default|SetAs%20GI%20SCP _asgi_scp))
  (if (Variables|/Game/Team7/Game/GI_SCP.GI_SCP_C|GetHasSuitcase _output_get)
    (Actor|DestroyActor)))

(event EventInteract
  ;[0.15 0.15 0.15 0.5] Add the mapping context with the IA Reset Run then destroys the actor
  (bind _asbp_first_person_character (Utilities|Casting|CastToBP_FirstPersonCharacter (Game|Player|GetPlayerPawn 0)))
  (Utilities|IsValid _asbp_first_person_character
    (:Is%20Valid
      (Default|CEAddMappingContext _asbp_first_person_character)
      (Actor|DestroyActor)
      (Variables|/Game/Team7/Game/GI_SCP.GI_SCP_C|SetHasSuitcase (Variables|Default|GetAs%20GI%20SCP) true))))

(event EventShowInteraction
  (params (InteractUI :type WBP%20Interaction%20Object%20Reference))
  (Default|SetInteractMessage InteractUI "Press [E] to pick up suitcase"))

(fn ConstructionScript)