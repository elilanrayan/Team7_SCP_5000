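; Death zone actor that restarts the level when an actor overlaps it.
; On overlap it disables that actor's input for player 0, without filtering by class, then calls the level reload with fade on the GI_SCP game instance cached at BeginPlay.
; The construction script sizes the box from BoxExtent and positions four arrows from that extent and the Scene component's relative location, along X and Z.
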(event EventBeginPlay
  (bind _asgi_scp (Utilities|Casting|CastToGI_SCP (Game|GetGameInstance)))
  (Variables|Default|SetAs%20GI%20SCP _asgi_scp))

(event Collision|EventActorBeginOverlap
  (params (OtherActor :type Actor%20Object%20Reference))
  (Input|DisableInput OtherActor (Game|GetPlayerController 0))
  (Default|CEReloadLevelwithFade (Variables|Default|GetAs%20GI%20SCP)))

(fn ConstructionScript
  (bind _scene (Variables|Default|GetScene))
  (bind _scene_2 (Variables|Default|GetScene))
  (bind _scene_3 (Variables|Default|GetScene))
  (bind _scene_4 (Variables|Default|GetScene))
  (bind _relativelocation (Variables|/Script/Engine.SceneComponent|GetRelativeLocation _scene))
  (bind _relativelocation_2 (Variables|/Script/Engine.SceneComponent|GetRelativeLocation _scene_3))
  (bind _relativelocation_3 (Variables|/Script/Engine.SceneComponent|GetRelativeLocation _scene_4))
  (bind _relativelocation_4 (Variables|/Script/Engine.SceneComponent|GetRelativeLocation _scene_2))
  (Components|Box|SetBoxExtent (Variables|Default|GetBox) (Variables|Default|GetBox%20Extent) true)
  (bind _result (Math|Float|NegateFloat (- (.z (Variables|Default|GetBox%20Extent)) (.z _relativelocation_3)))
    (:%20%20
      (Transformation|SetWorldLocation (Variables|Default|GetArrowBas) (Math|Vector|MakeVector (.x _relativelocation_3) (.y _relativelocation_3) _result) false false)
      (Transformation|SetWorldLocation (Variables|Default|GetArrowHaut) (Math|Vector|MakeVector (.x _relativelocation) (.y _relativelocation) (+ (.z _relativelocation) (.z (Variables|Default|GetBox%20Extent)))) false false)
      (bind _result_2 (Math|Float|NegateFloat (- (.x (Variables|Default|GetBox%20Extent)) (.x _relativelocation_2)))
        (:%20%20
          (Transformation|SetWorldLocation (Variables|Default|GetArrowLeft) (Math|Vector|MakeVector _result_2 (.y _relativelocation_2) (.z _relativelocation_2)) false false)
          (Transformation|SetWorldLocation (Variables|Default|GetArrowRight) (Math|Vector|MakeVector (+ (.x (Variables|Default|GetBox%20Extent)) (.x _relativelocation_4)) (.y _relativelocation_4) (.z _relativelocation_4)) false false))))))