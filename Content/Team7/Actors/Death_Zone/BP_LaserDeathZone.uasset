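; Laser death zone actor that procedurally builds a column of static meshes in the construction script; its event graph has no active logic.
; Spline points are stacked upward from the bottom arrow by Space, capped by the box's Z extent, and any overshoot snaps to the top arrow.
; A mesh component is added at each point, using the point's world-space location as its relative transform.
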(event EventBeginPlay
  (|CallParentFunction) ; This node is disabled and will not be called.\nDrag off pins to build functionality.
)

(event Collision|EventActorBeginOverlap
  (params (OtherActor :type Actor%20Object%20Reference))
  (|CallParentFunction OtherActor) ; This node is disabled and will not be called.\nDrag off pins to build functionality.
)

(event EventTick
  (params (DeltaSeconds :type Float%20%28single-precision%29)))

(fn ConstructionScript
  (bind _spline (Variables|Default|GetSpline))
  (bind _arrowhaut (Variables|Default|GetArrowHaut))
  (bind _arrowbas (Variables|Default|GetArrowBas))
  (bind _arrowbas_2 (Variables|Default|GetArrowBas))
  (bind _relativelocation (Variables|/Script/Engine.SceneComponent|GetRelativeLocation _arrowhaut))
  (bind _relativelocation_2 (Variables|/Script/Engine.SceneComponent|GetRelativeLocation _arrowbas_2))
  (bind _relativelocation_3 (Variables|/Script/Engine.SceneComponent|GetRelativeLocation _arrowbas))
  (|CallParentFunction)
  (Spline|ClearSplinePoints _spline true)
  (Spline|AddSplinePointatIndex _spline (Math|Vector|MakeVector (.x _relativelocation_2) (.y _relativelocation_2) (.z _relativelocation_2)) (Variables|Default|GetIndex) "Local" true)
  (Utilities|FlowControl|ForLoopwithBreak 0 (Math|Float|Truncate (.z (Variables|Default|GetBox%20Extent))) :!label _label
    (:LoopBody
      (if (> (.z (Spline|GetLocationatSplinePoint (Variables|Default|GetSpline) (Variables|Default|GetIndex) "Local")) (.z (Variables|/Script/Engine.SceneComponent|GetRelativeLocation (Variables|Default|GetArrowHaut))))
        (Spline|SetLocationatSplinePoint (Variables|Default|GetSpline) (Variables|Default|GetIndex) (Math|Vector|MakeVector (.x _relativelocation) (.y _relativelocation) (.z _relativelocation)) "Local" true)
        (goto _label Break)
        (else
          (bind _result (Math|Integer|IncrementInt (Variables|Default|GetIndex))
            (:%20%20
              (Spline|AddSplinePointatIndex _spline (Math|Vector|MakeVector (.x _relativelocation_3) (.y _relativelocation_3) (+ (.z _relativelocation_3) (* _result (Variables|Default|GetSpace)))) _result "Local" true))))))
    (:Completed
      (for _index (range 0 (Variables|Default|GetIndex))
        (bind _returnvalue (AddComponent|AddStaticMeshComponent false (Math|Conversions|ToTransform(Vector) (Spline|GetLocationatSplinePoint (Variables|Default|GetSpline) _index "World"))))
        (Components|StaticMesh|SetStaticMesh _returnvalue (Variables|Default|GetNew%20Mesh))))))