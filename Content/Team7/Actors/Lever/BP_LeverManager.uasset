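; Manager for a timed lever puzzle that destroys the BP_DoorbyLever door when solved.
; On BeginPlay it numbers the listed levers and binds their events, accepting them only in index order and deactivating out-of-order ones.
; The first valid pull starts a one-use Tick countdown, whose expiry resets lever states and locks out further attempts.
; VerifyAllLever checks completion by returning only the last lever's Activate flag.
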(event Custom|CE_ActivateTimer
  (params (Index :type Integer) (Lever :type BP%20Lever%20Object%20Reference))
  ;[0.15 0.15 0.15 0.5] Verify
  (if (Variables|Default|GetTimeOver)
    (Development|PrintString "Temps fini")
    (elif (== Index (Variables|Default|GetActivateLevel))
      (Math|Integer|IncrementInt (Variables|Default|GetActivateLevel)
        (:%20%20
          (bind _result (CallFunction|VerifyAllLever))
          (if _result
            (CallFunction|CEOpenDoor)
            (Variables|Default|SetAllLeverActivated true)
            (elif (not (Variables|Default|GetTimerAlreadyActivated))
              (Variables|Default|SetActivateTimer true)
              (Variables|Default|SetTimerAlreadyActivated true)))))
      (else
        (Default|CEDesactivate Lever)))))

(event Custom|CE_DesactivateAllLever
  ;[0.15 0.15 0.15 0.5] Fail Lever
  (for _array_element (Variables|Default|GetLever_List)
    (Variables|/Game/Team7/Actors/Lever/BP_Lever.BP_Lever_C|SetActivate _array_element false)
    (Development|PrintString "porte raté")))

(event Custom|CE_OpenDoor
  ;[0.15 0.15 0.15 0.5] Open_door
  (Development|PrintString "porte ouverte")
  (Default|CEDestroyME (Variables|Default|GetDoor)))

(event EventBeginPlay
  ;[0.15 0.15 0.15 0.5] Verify
  (bind _returnvalue (Actor|GetActorOfClass "/Game/Team7/Actors/Lever/BP_DoorbyLever.BP_DoorbyLever_C"))
  (Variables|Default|SetDoor _returnvalue)
  (for (_array_element _array_index) (Variables|Default|GetLever_List)
    (Variables|/Game/Team7/Actors/Lever/BP_Lever.BP_Lever_C|SetIndexNumber _array_element _array_index)
    (EventDispatchers|BindEventtoActivateTimer _array_element (delegate Custom|CE_ActivateTimer))))

(event EventTick
  (params (DeltaSeconds :type Float%20%28single-precision%29))
  ;[0.15 0.15 0.15 0.5] Timer Unique Usage
  (if (Variables|Default|GetActivateTimer)
    (bind _output_get (Variables|Default|SetTimer (- (Variables|Default|GetTimer) DeltaSeconds)))
    (if (<= _output_get 0.0)
      (Variables|Default|SetActivateTimer false)
      (if (not (Variables|Default|GetAllLeverActivated))
        (CallFunction|CEDesactivateAllLever)
        (Variables|Default|SetTimeOver true)))))

(fn ConstructionScript)

(fn VerifyAllLever
  (for _array_element (Variables|Default|GetLever_List)
    _)
  (return (Variables|/Game/Team7/Actors/Lever/BP_Lever.BP_Lever_C|GetActivate _array_element)))