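; BP_Fiche is an interactable sheet (fiche) prop that opens a full UI view of its own texture, although its prompt reads "enter password".
; On interact, it uses the HUD cached from GI_SCP at BeginPlay to create WBP_Fiche, pass it the texture and bind a close event.
; IsOpened hides the prompt while open, and closing returns to game through the HUD.
; The construction script applies the per-instance material to the cube.
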(event Custom|CE_CloseWidget
  ;[0.15 0.15 0.15 0.5] Close Password Widegt
  (Variables|Default|SetIsOpened (not (Variables|Default|GetIsOpened)))
  (if (Variables|Default|GetGI%20IsValid)
    (Default|CEReturntoGame (Variables|/Game/Team7/Game/GI_SCP.GI_SCP_C|GetHUD (Variables|Default|GetAs%20GI%20SCP)) (Variables|Default|GetFicheUI))))

(event EventBeginPlay
  ;[0.15 0.15 0.15 0.5] BeginPlay
  (bind _asgi_scp (Utilities|Casting|CastToGI_SCP (Game|GetGameInstance)))
  (bind _output_get (Variables|Default|SetAs%20GI%20SCP _asgi_scp))
  (if (!= _output_get 0)
    (Variables|Default|SetGI%20IsValid true)
    (else
      (Variables|Default|SetGI%20IsValid false))))

(event EventShowInteraction
  (params (InteractUI :type WBP%20Interaction%20Object%20Reference))
  ;[0.15 0.15 0.15 0.5] Show interaction message depending if the Password Widget is open
  (if (Variables|Default|GetIsOpened)
    (Default|SetInteractMessage InteractUI)
    (else
      (Default|SetInteractMessage InteractUI "Press [E] to enter password"))))

(event EventInteract
  (bind _as_gi_scp (Variables|Default|GetAs%20GI%20SCP))
  (bind _hud (Variables|/Game/Team7/Game/GI_SCP.GI_SCP_C|GetHUD _as_gi_scp))
  ;[0.15 0.15 0.15 0.5] Creating, setting up and opening Password Widget
  (Variables|Default|SetIsOpened (not (Variables|Default|GetIsOpened)))
  (if (Variables|Default|GetGI%20IsValid)
    (Default|CEInteractableUI _hud)
    (bind _wbpcreate (Default|FCreateWBP _hud "/Game/Team7/UI/WBP_Fiche.WBP_Fiche_C"))
    (bind _aswbp_fiche (Utilities|Casting|CastToWBP_Fiche _wbpcreate))
    (Variables|Default|SetFicheUI _aswbp_fiche)
    (EventDispatchers|BindEventtoCloseWidget (Variables|Default|GetFicheUI) (EventDispatchers|CreateEvent :!event Custom|CE_CloseWidget))
    (Default|CEFicheChanger (Variables|Default|GetFicheUI) (Variables|Default|GetficheTexture))))

(fn ConstructionScript
  (Rendering|Material|SetMaterial (Variables|Default|GetCube) 0 (Variables|Default|GetficheMaterial)))