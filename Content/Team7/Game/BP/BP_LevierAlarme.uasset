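; BP_LevierAlarme is an interactable lever that shuts off the alarm and reopens its linked door.
; On BeginPlay it gathers every BP_LightAlarme, registers itself with its alarm zones and opens the door.
; An activation event lights the alarms and closes and locks the door.
; Interacting calls deactivation, which zeroes light intensity and unlocks and opens the door, then clears the CanLightsOn flag.
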(event Custom|CE_AvtivateAllLights
  (bind _door (Variables|Default|GetDoor))
  (for _array_element (Variables|Default|GetLightsAlarme)
    (Rendering|Components|Light|SetIntensity (Variables|/Game/Team7/Game/BP/BP_LightAlarme.BP_LightAlarme_C|GetPointLight _array_element) 2e+03)
    (Variables|/Game/Team7/Actors/BP_Door.BP_Door_C|SetCanOpenDoor _door false)
    (Default|CECloseDoor _door)))

(event Custom|CE_DesactivateAllLights
  (bind _door (Variables|Default|GetDoor))
  (for _array_element (Variables|Default|GetLightsAlarme)
    (Rendering|Components|Light|SetIntensity (Variables|/Game/Team7/Game/BP/BP_LightAlarme.BP_LightAlarme_C|GetPointLight _array_element) 0.0)
    (Variables|/Game/Team7/Actors/BP_Door.BP_Door_C|SetCanOpenDoor _door true)
    (Default|CEOpenDoors _door)))

(event EventShowInteraction
  (params (InteractUI :type WBP%20Interaction%20Object%20Reference))
  (Default|SetInteractMessage InteractUI "Press [E] to interact with levier"))

(event EventInteract
  (CallFunction|CEDesactivateAllLights)
  (Variables|Default|SetCanLightsOn false))

(event EventBeginPlay
  (bind _outactors (Actor|GetAllActorsOfClass "/Game/Team7/Game/BP/BP_LightAlarme.BP_LightAlarme_C"))
  (Variables|Default|SetLightsAlarme _outactors)
  (Variables|Default|SetCanLightsOn true)
  (for _array_element (Variables|Default|GetZoneAlarme)
    (Variables|/Game/Team7/Game/BP/BP_ZoneAlarme.BP_ZoneAlarme_C|SetLevierAlarme _array_element self)
    (Default|CEOpenDoors (Variables|Default|GetDoor))))

(fn ConstructionScript)