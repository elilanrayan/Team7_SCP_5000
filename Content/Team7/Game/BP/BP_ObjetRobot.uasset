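; BP_ObjetRobot is a collectible object that the player picks up through interaction.
; On BeginPlay it caches the GI_SCP game instance and flags whether the reference is valid.
; It sets a take-object prompt on the interaction UI.
; On interact, if the reference is valid, it adds itself to the game instance's taken-item list, triggers the victory check, then destroys itself.
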(event EventBeginPlay
  ;[0.15 0.15 0.15 0.5] BeginPlay
  (bind _asgi_scp (Utilities|Casting|CastToGI_SCP (Game|GetGameInstance)))
  (bind _output_get (Variables|Default|SetAs%20GI%20SCP _asgi_scp))
  (if (!= _output_get 0)
    (Variables|Default|SetGI%20IsValid true)
    (else
      (Variables|Default|SetGI%20IsValid false))))

(event EventShowInteraction
  (params (InteractUI :type WBP%20Interaction%20Object%20Reference))
  (Default|SetInteractMessage InteractUI "Press [E] to take object"))

(event EventInteract
  (bind _as_gi_scp (Variables|Default|GetAs%20GI%20SCP))
  (if (Variables|Default|GetGI%20IsValid)
    (Utilities|Array|Add (Variables|/Game/Team7/Game/GI_SCP.GI_SCP_C|GetListItemTake _as_gi_scp) self)
    (Default|CECheckVictory _as_gi_scp)
    (Actor|DestroyActor)))

(fn ConstructionScript)