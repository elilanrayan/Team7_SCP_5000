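; BP_Robot is an interactable robot that shows how many of three pieces the player has recovered.
; On BeginPlay it casts the game instance to GI_SCP, caches it and records whether the reference is valid.
; Its ShowInteraction event sets the interaction UI message to a French progress text, using the length of the game instance's ListItemTake as the count, without checking the validity flag.
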(event EventBeginPlay
  ;[0.15 0.15 0.15 0.5] BeginPlay
  (bind _asgi_scp (Utilities|Casting|CastToGI_SCP (Game|GetGameInstance)))
  (bind _output_get (Variables|Default|SetAs%20GI%20SCP _asgi_scp))
  (if (!= _output_get 0)
    (Variables|Default|SetGI%20IsValid true)
    (else
      (Variables|Default|SetGI%20IsValid false))))

(event EventShowInteraction
  (params (InteractUI :type WBP%20Interaction%20Object%20Reference))
  (Default|SetInteractMessage InteractUI (Utilities|Text|FormatText "Nombre de pieces recuperer : {numListe} / 3" (Utilities|Array|Length (Variables|/Game/Team7/Game/GI_SCP.GI_SCP_C|GetListItemTake (Variables|Default|GetAs%20GI%20SCP))))))

(fn ConstructionScript)